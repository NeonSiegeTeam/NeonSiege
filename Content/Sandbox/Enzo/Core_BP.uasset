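; Destructible core for the Neon Siege game mode that bobs vertically on a sine wave and ends the round when destroyed.
; Projectile hits, throttled by a short cooldown, apply negative damage that feeds the health component's Modify.
; The health ratio drives a Life material parameter on the core mesh.
; On death it activates an explosion, hides the mesh and calls RoundEnded(false) on the game mode.
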(event `self.ReceiveBeginPlay`
  (set `self.initial Position` (`SceneComponent.K2_GetComponentLocation` (`self.Core_SM`))))

(event `self.ReceiveTick`
  (params (DeltaSeconds :type "Float (single-precision)"))
  (`SceneComponent.K2_SetWorldLocation` (`self.Core_SM`) (+ (`self.initial Position`) (* (`KismetMathLibrary.Vector_Up`) (`KismetMathLibrary.Sin` (`GameplayStatics.GetTimeSeconds`)) 100)) false false))

(event `self.ReceiveAnyDamage`
  (params (Damage :type "Float (single-precision)") (DamageType :type "DamageType Object Reference") (InstigatedBy :type "Controller Object Reference") (DamageCauser :type "Actor Object Reference"))
  (bind _health_ac (`self.Health_AC`))
  (`/Game/Sandbox/Enzo/Health_AC.Modify` _health_ac Damage)
  (`self.UpdateHealthDisplay` (`/Game/Sandbox/Enzo/Health_AC.Ratio` _health_ac)))

(event `self.Core_SM.OnComponentHit`
  (params (HitComponent :type "PrimitiveComponent Object Reference") (OtherActor :type "Actor Object Reference") (OtherComp :type "PrimitiveComponent Object Reference") (NormalImpulse :type "Vector Structure") (Hit :type "HitResult Structure (by ref)"))
  (bind _returnvalue (`GameplayStatics.GetTimeSeconds`))
  (cast `/Game/MobileBlueprints/Projectiles/Projectiles_BP` OtherActor)
  (if (> _returnvalue (+ (`self.lasthit`) 0.5))
    (set `self.lasthit` _returnvalue)
    (`GameplayStatics.ApplyDamage` self -1.0)))

(event `UpdateHealthDisplay`
  (params (Ratio :type "Float (single-precision)"))
  (`MeshComponent.SetScalarParameterValueOnMaterials` (`self.Core_SM`) "Life" Ratio))

(event `self.Health_AC.Die`
  ;[0.2302 0 0.1302 0.308] End game if destroyed
  (`self.Core Explosion`)
  (bind _asneon_siege_game_mode (cast `/Game/GameModes/NeonSiegeGameMode` (`GameplayStatics.GetGameMode`)))
  (`/Game/GameModes/NeonSiegeGameMode.RoundEnded` _asneon_siege_game_mode false))

(event `Core Explosion`
  (`ActorComponent.Activate` (`self.CoreExplosion`) true)
  (`SceneComponent.SetVisibility` (`self.Core_SM`) false false))

(fn `UserConstructionScript`)