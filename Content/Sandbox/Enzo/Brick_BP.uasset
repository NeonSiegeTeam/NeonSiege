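; Destructible physics brick that loses health when struck by projectiles, with a short cooldown between hits.
; Damage feeds a health component, whose ratio drives the outline's Life material parameter alongside a blink effect and damage notification.
; Death hides the cube, disables its physics and collision, plays a dissolve effect sized from cube scale, then destroys the actor.
; The authority triggers multicast damage and disintegration sounds with randomized pitch.
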(event `self.ReceiveBeginPlay`
  (bind _health_ac (`self.Health_AC`))
  ;[1 1 1] Health
  (`/Engine/EditorBlueprintResources/ActorMacros.Switch Has Authority`
    (:`Authority`
      _)
    (:`Remote`
      _))
  (add `/Game/Sandbox/Enzo/Health_AC.Born` _health_ac (delegate `Born`))
  (add `/Game/Sandbox/Enzo/Health_AC.Die` _health_ac (delegate `Die`)))

(event `Born`
  ;[1 1 1] Health
  (`SceneComponent.SetVisibility` (`self.Cube`) true false)
  (`SceneComponent.SetVisibility` (`self.Outline`) true false))

(event `Die`
  ;[1 1 1] Health
  (`self.Fadeout`)
  (`self.DesintegrationSound`))

(event `self.ReceiveAnyDamage`
  (params (Damage :type "Float (single-precision)") (DamageType :type "DamageType Object Reference") (InstigatedBy :type "Controller Object Reference") (DamageCauser :type "Actor Object Reference"))
  (bind _health_ac (`self.Health_AC`))
  ;[1 1 1] Health
  (`/Game/Sandbox/Enzo/Health_AC.Modify` _health_ac Damage)
  (`self.UpdateHealthDisplay` (`/Game/Sandbox/Enzo/Health_AC.Ratio` _health_ac))
  (`self.DamageTaken`)
  (`self.Damage Sound`))

(event `Fadeout`
  ;[1 1 1] Health
  (`SceneComponent.SetVisibility` (`self.Cube`) false false)
  (`SceneComponent.SetVisibility` (`self.Outline`) false false)
  (`ActorComponent.Activate` (`self.Disolve`) true)
  (`PrimitiveComponent.SetSimulatePhysics` (`self.Cube`) false)
  (`PrimitiveComponent.SetCollisionEnabled` (`self.Cube`) "NoCollision")
  (`KismetSystemLibrary.Delay` 2.0)
  (`self.K2_DestroyActor`))

(event `self.Cube.OnComponentHit`
  (params (HitComponent :type "PrimitiveComponent Object Reference") (OtherActor :type "Actor Object Reference") (OtherComp :type "PrimitiveComponent Object Reference") (NormalImpulse :type "Vector Structure") (Hit :type "HitResult Structure (by ref)"))
  (bind _returnvalue (`GameplayStatics.GetTimeSeconds`))
  ;[1 1 1] Health
  (cast `/Game/MobileBlueprints/Projectiles/Projectiles_BP` OtherActor)
  (if (> _returnvalue (+ (`self.lasthit`) 0.5))
    (set `self.lasthit` _returnvalue)
    (`GameplayStatics.ApplyDamage` self -1.0)))

(event `UpdateHealthDisplay`
  (params (HealthRatio :type "Float (double-precision)"))
  ;[1 1 1] Health
  (`MeshComponent.SetScalarParameterValueOnMaterials` (`self.Outline`) "Life" HealthRatio)
  (`ActorComponent.Activate` (`self.CubeBlink`) true))

(event `Damage Sound`
  ;[0.1084 0 0.2344 0.178] Damage sound
  (`/Engine/EditorBlueprintResources/ActorMacros.Switch Has Authority`
    (:`Authority`
      (`self.MC_ Damage Sound`))))

(event `MC_ Damage Sound`
  ;[0.1084 0 0.2344 0.178] Damage sound
  (bind _pitch (`/Game/Assets/Sounds/SoundFunctions.GetRandomPitch` 0.9 1.1))
  (`GameplayStatics.PlaySoundAtLocation` "/Game/Assets/Sounds/Effects/damageBlock1.damageBlock1" (`self.K2_GetActorLocation`) (struct) 1.0 _pitch 0.0 (`self.Attenuation`) null null null))

(event `DesintegrationSound`
  ;[0.1084 0 0.2344 0.178] Desintegration sound
  (`/Engine/EditorBlueprintResources/ActorMacros.Switch Has Authority`
    (:`Authority`
      (`self.MC_DesintegrationSound`))))

(event `MC_DesintegrationSound`
  ;[0.1084 0 0.2344 0.178] Desintegration sound
  (bind _pitch (`/Game/Assets/Sounds/SoundFunctions.GetRandomPitch` 0.9 1.1))
  (`GameplayStatics.PlaySoundAtLocation` "/Game/Assets/Sounds/Effects/explosionBlock.explosionBlock" (`self.K2_GetActorLocation`) (struct) 1.0 _pitch 0.0 (`self.Attenuation`) null null null))

(fn `UserConstructionScript`
  (bind (_returnvalue_x _returnvalue_y _returnvalue_z) (`KismetMathLibrary.BreakVector` (`SceneComponent.K2_GetComponentScale` (`self.Cube`))))
  (`SceneComponent.SetWorldScale3D` (`self.Disolve`) (1.0 1.0 1.0))
  (`|ExecutionSequence`
    (:`then_0`
      (`NiagaraComponent.SetVariableInt` (`self.Disolve`) "ScaleX" (`KismetMathLibrary.FTrunc` _returnvalue_x)))
    (:`then_1`
      (`NiagaraComponent.SetVariableInt` (`self.Disolve`) "ScaleY" (`KismetMathLibrary.FTrunc` _returnvalue_y)))
    (:`then_2`
      (`NiagaraComponent.SetVariableInt` (`self.Disolve`) "ScaleZ" (`KismetMathLibrary.FTrunc` _returnvalue_z)))))