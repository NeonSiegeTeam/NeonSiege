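; Base-style projectile Blueprint with a server-controlled lifetime and a sound for hits on shields.
; Throw launches the Sphere with a velocity-change impulse.
; The server destroys the actor on Tick once Lifetime elapses, and on the first Sphere hit against a Shield_VFX actor calls MC_ShieldSound.
; That event, apparently a multicast, plays an attenuated, randomly pitched block sound at the projectile's location.
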(event `self.ReceiveBeginPlay`
  ;[1 1 1] Lifetime
  (`/Engine/EditorBlueprintResources/ActorMacros.Switch Has Authority`
    (:`Authority`
      (set `self.StartTime` (`GameplayStatics.GetTimeSeconds`)))))

(event `self.ReceiveTick`
  (params (DeltaSeconds :type "Float (single-precision)"))
  ;[1 1 1] Lifetime
  (`/Engine/EditorBlueprintResources/ActorMacros.Switch Has Authority`
    (:`Authority`
      (if (> (- (`GameplayStatics.GetTimeSeconds`) (`self.StartTime`)) (`self.Lifetime`))
        (`self.K2_DestroyActor`)))))

(event `self.Sphere.OnComponentHit`
  (params (HitComponent :type "PrimitiveComponent Object Reference") (OtherActor :type "Actor Object Reference") (OtherComp :type "PrimitiveComponent Object Reference") (NormalImpulse :type "Vector Structure") (Hit :type "HitResult Structure (by ref)"))
  ;[0.1084 0 0.2344 0.178] Shield block
  (`/Engine/EditorBlueprintResources/ActorMacros.Switch Has Authority`
    (:`Authority`
      (cast `/Game/PCBlueprints/Features/Shield/Shield_VFX` OtherActor)
      (if (not (`self.hasPlayedSound`))
        (set `self.hasPlayedSound` true)
        (`self.MC_ShieldSound`)))))

(event `MC_ShieldSound`
  ;[0.1084 0 0.2344 0.178] Shield block
  (bind _pitch (`/Game/Assets/Sounds/SoundFunctions.GetRandomPitch` 0.9 1.1))
  (`GameplayStatics.PlaySoundAtLocation` "/Game/Assets/Sounds/Effects/Pulse/Shield_Block.Shield_Block" (`self.K2_GetActorLocation`) (struct) 1.0 _pitch 0.0 (`self.Attenuation`) null null null))

(fn `Throw`
  (params (Force :type "Vector Structure"))
  (`PrimitiveComponent.AddImpulse` (`self.Sphere`) Force "None" true))

(fn `UserConstructionScript`)