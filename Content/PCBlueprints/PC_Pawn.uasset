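; PC pawn that spawns Brick_BP actors from its BrickSpawner component, either singly or as whole walls, each on its own cooldown.
; SpawnBrick drops one brick at a random point along the spawner's forward axis.
; BuildAWall uses a custom ForLoopWithDelay macro to spawn timed rows brick by brick along that axis, all at spawner height.
; Rows alternate between full and one brick short, with a shifted start for a staggered bond.
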(event `Add Offset`
  ;[0.1084 0 0.2344 0.178] Add offset
  (set `self.CurrentPos` (+ (`self.CurrentPos`) (* (`self.Direction`) (.x (`SceneComponent.K2_GetComponentScale` (`self.BrickSpawner`))) 50))))

(event `Switch`
  ;[0.1084 0 0.2344 0.178] Switch
  (set `self.IsRowFull` (not (`self.IsRowFull`))))

(event `Reset Offset`
  (params (IsRowFull :type Boolean))
  (bind _direction (`self.Direction`))
  (bind _returnvalue (+ (.location (`self.StartTransform`)) (* _direction -100 (.x (`SceneComponent.K2_GetComponentScale` (`self.BrickSpawner`))))))
  ;[0.1084 0 0.2344 0.178] Reset Offset
  (if IsRowFull
    (set `self.CurrentPos` _returnvalue)
    (else
      (set `self.CurrentPos` (+ _returnvalue (* _direction 300))))))

(event `Build a segment`
  (params (Full :type Boolean))
  ;[0.1084 0 0.2344 0.178] Build a segment
  (if Full
    (`self.For Loop With Delay` 1 (`self.BrickPerRow`) 0.1
      (:`Loop`
        (`|SpawnActorFromClass` "/Game/Sandbox/Enzo/Brick_BP.Brick_BP_C" (`KismetMathLibrary.MakeTransform` (`self.CurrentPos`) (.rotation (`self.StartTransform`)) (4.0 2.0 2.0)) "AdjustIfPossibleButAlwaysSpawn" "MultiplyWithRoot" null null :!label _label)
        (`self.Add Offset`))
      (:`Completed`
        (`self.Reset Offset` (`self.IsRowFull`) :!label _label_2)))
    (else
      (`self.For Loop With Delay` 1 (- (`self.BrickPerRow`) 1) 0.1
        (:`Loop`
          (goto _label))
        (:`Completed`
          (goto _label_2))))))

(event `Build A Wall`
  (bind _returnvalue (`GameplayStatics.GetTimeSeconds`))
  (bind _brickspawner (`self.BrickSpawner`))
  ;[0.1084 0 0.2344 0.178] Global Cooldwon
  (if (<= (+ (`self.LastWallBuild`) (`self.GlobalCooldown`)) _returnvalue)
    (set `self.LastWallBuild` _returnvalue)
    (set `self.IsRowFull` true)
    (bind _output_get (set `self.StartTransform` (`SceneComponent.K2_GetComponentToWorld` _brickspawner)))
    (bind _output_get_2 (set `self.Direction` (`SceneComponent.GetForwardVector` _brickspawner)))
    (set `self.CurrentPos` (+ (.location _output_get) (* _output_get_2 -100 (.x (`SceneComponent.K2_GetComponentScale` (`self.BrickSpawner`))))))
    (`self.For Loop With Delay` 1 (`self.NumberOfSegment`) 0.6
      (:`Loop`
        (`self.Build a segment` (`self.IsRowFull`))
        (`self.Switch`)))))

(event `Spawn Brick`
  (bind _returnvalue (`GameplayStatics.GetTimeSeconds`))
  ;[0.1084 0 0.2344 0.178] Cooldown
  (if (< (+ (`self.LastBrickSpawned`) (`self.SpawnCooldown`)) _returnvalue)
    (set `self.LastBrickSpawned` _returnvalue)
    ;[0.1084 0 0.2344 0.178] Spawn brick
    (bind _position (`self.Get Random Brick Pos`))
    (`|SpawnActorFromClass` "/Game/Sandbox/Enzo/Brick_BP.Brick_BP_C" (`KismetMathLibrary.MakeTransform` _position (.rotation (`SceneComponent.K2_GetComponentToWorld` (`self.BrickSpawner`))) (4.0 2.0 2.0)) "Undefined" "MultiplyWithRoot" null null)))

(fn `Get Random Brick Pos`
  (returns (position :type "Vector Structure"))
  (bind _brickspawner (`self.BrickSpawner`))
  (bind _x (.x (`SceneComponent.K2_GetComponentScale` _brickspawner)))
  (return (+ (`SceneComponent.K2_GetComponentLocation` _brickspawner) (* (`SceneComponent.GetForwardVector` _brickspawner) (* (`KismetMathLibrary.RandomFloatInRange` (- 0.0 _x) _x) 50.0)))))

(fn `UserConstructionScript`)